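; Player character Blueprint for the skater Skye, routing input to components for running, jumping, grinding, wall catching and camera handling.
; Tick applies uphill multipliers to running, widens FOV with speed, and drops the skater into Falling when slow and tilted away from Ninja movement's gravity-up.
; BeginPlay wires grind audio, blob shadow, landing sound, and speed-line and skate-trail effects for SenseOfSpeedComponent.
; P saves player state; L loads it through SaveState components.
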(event Custom|AdjustHitboxSize
  (Components|Capsule|SetCapsuleHalfHeight (Variables|Default|GetCapsuleComponent) 48.0 true))

(event Custom|PlayLandedSound
  (Audio|PlaySoundatLocation "/Game/Audio/SFX/SkatesJump_Cue.SkatesJump_Cue" (Transformation|GetActorLocation) "0, 0, 0" 1.0 1.0 0.0 0 0 0))

(event EventBeginPlay
  (bind _blobshadow (Variables|Default|GetBlobShadow))
  (Variables|/Game/Blueprints/CharacterAbilities/GrindComponent.GrindComponent_C|SetMesh (Variables|Default|GetGrindComponent) (Variables|Character|GetMesh))
  (EventDispatchers|BindEventtoPreparetoJump (Variables|Default|GetJumpQoLComponent) (EventDispatchers|CreateEvent (Variables|Default|GetGrindComponent) :!event StopGrinding))
  (CallFunction|InitSpeedlines)
  (CallFunction|InitSkateTrailsParticle)
  (bind _output_get (Variables|/Game/Blueprints/CharacterAbilities/GrindComponent.GrindComponent_C|SetGrindSound (Variables|Default|GetGrindComponent) (Variables|Default|GetGrindAudio)))
  (Components|Activation|Deactivate _output_get)
  (Variables|/Game/Blueprints/CharacterAbilities/BlobShadow.BlobShadow_C|SetShadow _blobshadow (Variables|Default|GetDecal))
  (Variables|/Game/Blueprints/CharacterAbilities/BlobShadow.BlobShadow_C|SetEmptyPlaceholder _blobshadow (Variables|Default|GetCube))
  (EventDispatchers|BindEventtoOnOwnerLanded (Variables|Default|GetStateInformation) (delegate Custom|PlayLandedSound)))

(event EventTick
  (params (DeltaSeconds :type Float%20%28single-precision%29))
  (bind _runcomponent (Variables|Default|GetRunComponent))
  (bind _uphillcomponent (Variables|Default|GetUphillComponent))
  (bind _mul (Variables|/Game/Blueprints/UphillComponent.UphillComponent_C|GetMul _uphillcomponent))
  (Variables|/Game/Blueprints/CharacterAbilities/RunComponent.RunComponent_C|SetSpeedMultiplier _runcomponent _mul)
  (Variables|/Game/Blueprints/CharacterAbilities/RunComponent.RunComponent_C|SetAccelMultiplier _runcomponent _mul)
  (bind _asninja_character_movement_component (Utilities|Casting|CastToNinjaCharacterMovementComponent (Variables|Character|GetCharacterMovement)))
  (if (and (< (Math|Vector|VectorLength (Variables|/Script/Engine.MovementComponent|GetVelocity (Variables|Character|GetCharacterMovement))) 8e+02) (< (Math|Vector|DotProduct (Transformation|GetActorUpVector) (* (Class|NinjaCharacterMovementComponent|GetGravityDirection _asninja_character_movement_component false) -1.0)) 0.9))
    (Pawn|Components|CharacterMovement|SetMovementMode (Variables|Character|GetCharacterMovement) "MOVE_Falling" 0))
  (Camera|SetFieldOfView (Variables|Default|GetFollowCamera) (Math|Float|Lerp 8e+01 1e+02 (/ (Math|Vector|VectorLength (Variables|/Script/Engine.MovementComponent|GetVelocity _asninja_character_movement_component)) 4e+03))))

(event Collision|EventHit
  (params (MyComp :type Primitive%20Component%20Object%20Reference) (Other :type Actor%20Object%20Reference) (OtherComp :type Primitive%20Component%20Object%20Reference) (bSelfMoved :type Boolean) (HitLocation :type Vector :default "0, 0, 0") (HitNormal :type Vector :default "0, 0, 0") (NormalImpulse :type Vector :default "0, 0, 0") (Hit :type Hit%20Result%20Structure%20%28by%20ref%29))
  (bind _asninja_character_movement_component (Utilities|Casting|CastToNinjaCharacterMovementComponent (Variables|Character|GetCharacterMovement)))
  (Default|Hit (Variables|Default|GetCatchWallComponent) HitNormal _asninja_character_movement_component)
  (Variables|Default|SetLandedThisFrame true)
  (Variables|Default|SetNewVar_1 2)
  (Variables|Default|Setdebuf (Transformation|GetActorLocation)))

(event Collision|EventActorBeginOverlap
  (params (OtherActor :type Actor%20Object%20Reference))
  (bind _asgrind_rail (Utilities|Casting|CastToGrindRail OtherActor))
  (Default|StartGrinding (Variables|Default|GetGrindComponent) _asgrind_rail))

(event EventRestartAnim
  (Variables|Default|SetHoldAnim false)
  (bind _asskater_skye_abp (Utilities|Casting|CastToSkaterSkye_ABP (Components|SkeletalMesh|GetAnimInstance (Variables|Character|GetMesh))))
  (Variables|/Game/Skater_Skye/SkaterSkye_ABP.SkaterSkye_ABP_C|SetholdSpeed _asskater_skye_abp 2.0))

(event EventPauseAnim
  (Variables|Default|SetHoldAnim true)
  (bind _asskater_skye_abp (Utilities|Casting|CastToSkaterSkye_ABP (Components|SkeletalMesh|GetAnimInstance (Variables|Character|GetMesh))))
  (Variables|/Game/Skater_Skye/SkaterSkye_ABP.SkaterSkye_ABP_C|SetholdSpeed _asskater_skye_abp (Math|Float|Lerp 1.1 0.5 (/ (Math|Vector|VectorLength (Variables|/Script/Engine.MovementComponent|GetVelocity (Variables|Character|GetCharacterMovement))) 4e+03))))

(event EventLoadState
  (params (SaveState :type Save%20State%20Component%20Object%20Reference))
  (bind _rotation (Variables|/Game/Blueprints/SaveStateComponent.SaveStateComponent_C|GetRotation SaveState))
  (Transformation|SetActorLocationAndRotation (Variables|/Game/Blueprints/SaveStateComponent.SaveStateComponent_C|GetLocation SaveState) _rotation false true)
  (bind _asplayer_save_state (Utilities|Casting|CastToPlayerSaveState SaveState))
  (Variables|/Script/Engine.MovementComponent|SetVelocity (Pawn|GetMovementComponent) (Variables|/Game/Data/PlayerSaveState.PlayerSaveState_C|GetVelocity _asplayer_save_state))
  (Default|ResetCamera (Variables|Default|GetHandleAutoManualCamera))
  (Pawn|SetControlRotation (Pawn|GetController) _rotation))

(event Input|ActionEvents|InputActionJump
  (params (Key :type Key%20Structure :default "None"))
  (bind _jumpqolcomponent (Variables|Default|GetJumpQoLComponent))
  (:Pressed
    (Default|AttempttoJump _jumpqolcomponent))
  (:Released
    (Default|ReleaseJump _jumpqolcomponent)))

(event Input|ActionEvents|InputActionBrake
  (params (Key :type Key%20Structure :default "None"))
  (bind _crouch1 (Variables|Default|GetCrouch1))
  (bind _runcomponent (Variables|Default|GetRunComponent))
  (:Pressed
    (Variables|/Game/Blueprints/CharacterAbilities/RunComponent.RunComponent_C|SetCanMove _runcomponent false)
    (Variables|/Game/Crouch.Crouch_C|SetCrouching _crouch1 true)
    (Variables|/Game/Blueprints/CharacterAbilities/RunComponent.RunComponent_C|SetTurnRate _runcomponent 4.0))
  (:Released
    (Variables|/Game/Blueprints/CharacterAbilities/RunComponent.RunComponent_C|SetCanMove _runcomponent true)
    (Variables|/Game/Crouch.Crouch_C|SetCrouching _crouch1 false)
    (Variables|/Game/Blueprints/CharacterAbilities/RunComponent.RunComponent_C|SetTurnRate _runcomponent 1.0)))

(event Input|ActionEvents|InputActionWallCatch
  (params (Key :type Key%20Structure :default "None"))
  (:Pressed
    (Default|SetReadytoCatch (Variables|Default|GetCatchWallComponent))))

(event Input|AxisEvents|InputAxisMoveForward
  (params (AxisValue :type Float%20%28single-precision%29))
  (Default|InputY (Variables|Default|GetRunComponent) AxisValue))

(event Input|AxisEvents|InputAxisMoveRight
  (params (AxisValue :type Float%20%28single-precision%29))
  (Default|InputX (Variables|Default|GetRunComponent) AxisValue))

(event Input|AxisEvents|InputAxisLookUp
  (params (AxisValue :type Float%20%28single-precision%29))
  (Pawn|Input|AddControllerPitchInput AxisValue)
  (if (!= AxisValue 0.0)
    (Default|CameraHasMovedManually (Variables|Default|GetHandleAutoManualCamera))))

(event Input|AxisEvents|InputAxisTurn
  (params (AxisValue :type Float%20%28single-precision%29))
  (Pawn|Input|AddControllerYawInput AxisValue)
  (if (!= AxisValue 0.0)
    (Default|CameraHasMovedManually (Variables|Default|GetHandleAutoManualCamera))))

(event Input|KeyboardEvents|F
  (params (Key :type Key%20Structure :default "None")))

(event Input|KeyboardEvents|H
  (params (Key :type Key%20Structure :default "None"))
  (:Pressed
    (EventDispatchers|BindEventtoJumpDispatcher (Variables|Default|GetJumpQoLComponent) (delegate Custom|AdjustHitboxSize))))

(event Input|KeyboardEvents|U
  (params (Key :type Key%20Structure :default "None")))

(event Input|KeyboardEvents|V
  (params (Key :type Key%20Structure :default "None")))

(event Input|KeyboardEvents|P
  (params (Key :type Key%20Structure :default "None"))
  (:Pressed
    (Default|SavePlayer (Variables|Default|GetPlayerSaveState) (Transformation|GetActorLocation) (Transformation|GetActorRotation) (Transformation|GetVelocity) (Pawn|GetControlRotation :!class /Script/Engine.Pawn))))

(event Input|KeyboardEvents|L
  (params (Key :type Key%20Structure :default "None"))
  (:Pressed
    (for _array_element (Actor|GetComponentsByClass "/Game/Blueprints/SaveStateComponent.SaveStateComponent_C")
      (Default|Load _array_element 0 "0, 0, 0" "0, 0, 0"))))

(fn ConstructionScript
  (|CallParentFunction))

(fn EnableStickyGravity
  (bind _asninja_character_movement_component (Utilities|Casting|CastToNinjaCharacterMovementComponent (Variables|Character|GetCharacterMovement)))
  (Variables|/Script/NinjaCharacter.NinjaCharacterMovementComponent|SetbAlignComponentToFloor _asninja_character_movement_component true)
  (Variables|/Script/NinjaCharacter.NinjaCharacterMovementComponent|SetbAlignComponentToGravity _asninja_character_movement_component false))

(fn SetSpeedlines
  (params (NewParam :type Float%20%28single-precision%29))
  (Rendering|Material|SetScalarParameterValue (Variables|Default|GetMyPPMat) "CenterSize" NewParam :!class /Script/Engine.MaterialInstanceDynamic))

(fn InitSpeedlines
  (bind _outactors (Actor|GetAllActorsOfClass "/Script/Engine.PostProcessVolume"))
  (Utilities|IsValid (Variables|Default|GetMyPPMat)
    (:Is%20Valid
      _)
    (:Is%20Not%20Valid
      (bind _returnvalue (Rendering|Material|CreateDynamicMaterialInstance "/Game/SpeedLinesInstance.SpeedLinesInstance" "None" "None" :!class /Script/Engine.KismetMaterialLibrary))
      (bind _output_get (Variables|Default|SetMyPPMat _returnvalue))))
  (Utilities|Array|Add (Utilities|Struct|BreakWeightedBlendables (Utilities|Struct|BreakPostProcessSettings (Variables|/Script/Engine.PostProcessVolume|GetSettings (Utilities|Array|Get(acopy) _outactors)))) (Utilities|Struct|MakeWeightedBlendable 1.0 _output_get))
  (Utilities|Struct|SetmembersinPostProcessSettings (Variables|/Script/Engine.PostProcessVolume|GetSettings (Utilities|Array|Get(acopy) _outactors)) (Utilities|Struct|MakeWeightedBlendables (Utilities|Struct|BreakWeightedBlendables (Utilities|Struct|BreakPostProcessSettings (Variables|/Script/Engine.PostProcessVolume|GetSettings (Utilities|Array|Get(acopy) _outactors))))))
  (Variables|/Game/SenseOfSpeedComponent.SenseOfSpeedComponent_C|SetSpeedLines (Variables|Default|GetSenseOfSpeedComponent) _output_get))

(fn InitSkateTrailsParticle
  (bind _senseofspeedcomponent (Variables|Default|GetSenseOfSpeedComponent))
  (bind _mesh (Variables|Character|GetMesh))
  (bind _returnvalue (Niagara|SpawnSystemAttached "/Game/SkatesTrails.SkatesTrails" _mesh "DEF-foot_L" "0, 0, 0" "0, 0, 0" "KeepRelativeOffset" false))
  (bind _returnvalue_2 (Niagara|SpawnSystemAttached "/Game/SkatesTrails.SkatesTrails" _mesh "DEF-foot_R" "0, 0, 0" "0, 0, 0" "KeepRelativeOffset" false))
  (Variables|/Game/SenseOfSpeedComponent.SenseOfSpeedComponent_C|SetSkatesTrailLeft _senseofspeedcomponent _returnvalue)
  (Variables|/Game/SenseOfSpeedComponent.SenseOfSpeedComponent_C|SetSkatesTrailRight _senseofspeedcomponent _returnvalue_2)
  (Effects|Components|ParticleSystem|SetColorParameter _returnvalue_2 "Color" "(R=1.000000,G=0.323075,B=0.000000,A=1.000000)"))

(fn ParticlesUpdate)

(fn UpdateHitboxSize
  (params (Grounded :type Boolean))
  (bind _returnvalue (Math|Float|SelectFloat 96.0 48.0 Grounded))
  (Components|Capsule|SetCapsuleHalfHeight (Variables|Default|GetCapsuleComponent) _returnvalue true)
  (if (!= _returnvalue (Variables|Default|GetCapsuleSavedSize))
    (bind _output_get (Variables|Default|SetCapsuleSavedSize _returnvalue))
    (if (and (> _output_get 5e+01) (Variables|Default|GetLandedThisFrame))
      (Transformation|SetActorLocation (+ (Transformation|GetActorLocation) (Math|Vector|MakeVector 0.0 0.0 (/ (Components|Capsule|GetScaledCapsuleHalfHeight (Variables|Default|GetCapsuleComponent)) 2.0))) false true)
      (else
        (Variables|Default|SetLandedThisFrame true)))))

(fn GetFootLocation
  (params (Left :type Boolean))
  (return "0, 0, 0"))

(fn GetMeshes
  (return 0 0 0 0 0 0 0))

(fn GetPlayerVelocity
  (return "0, 0, 0"))

(fn GetSpeed
  (return 0.0))

(fn ICanJump
  (bind _charactermovement (Variables|Character|GetCharacterMovement))
  (bind _returnvalue (AI|Components|NavMovement|IsFalling _charactermovement))
  (bind _returnvalue_2 (not _returnvalue))
  (CallFunction|UpdateHitboxSize _returnvalue_2)
  (return (or _returnvalue_2 (Utilities|IsValid (Variables|/Game/Blueprints/CharacterAbilities/GrindComponent.GrindComponent_C|GetGrind%20Rail%20Reference (Variables|Default|GetGrindComponent))))))

(fn IsNotonAWall
  (return false))