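; SaveStateComponent is an actor component that holds one saved location and rotation for state save and restore.
; Save stores the transform passed to it, and LoadF returns the stored values.
; Load ignores its inputs and sends LoadStateMessage to the owner with itself as the argument, leaving the owner to handle restoration.
; A teleporting SetActorLocationAndRotation node is left unconnected and never runs.
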(event Custom|Save
  (params (NewParam :type Vector) (NewParam2 :type Rotator))
  (Variables|Default|SetLocation NewParam)
  (Variables|Default|SetRotation NewParam2))

(event Custom|Load
  (params (NewParam :type Actor%20Object%20Reference) (NewParam2 :type Rotator) (NewParam3 :type Rotator))
  (Class|SaveStateInterface|LoadState(Message) (Components|GetOwner) self))

(event EventBeginPlay)

(event EventTick
  (params (DeltaSeconds :type Float%20%28single-precision%29)))

(fn LoadF
  (return (Variables|Default|GetLocation) (Variables|Default|GetRotation)))