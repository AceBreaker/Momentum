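; Character component that adds a ground drift move, started while drift input is held with horizontal input and stopped when the character falls.
; Each tick while drifting it zeroes ground friction, keeps speed while angling velocity off the forward vector, and yaws the character in the locked drift direction.
; Horizontal input adjusts the turn rate.
; Start and stop toggle the KinzieAnimBP drift flag and message the owner for effects.
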(event EventBeginPlay
  (bind _ascharacter (Utilities|Casting|CastToCharacter (Components|GetOwner)))
  (Variables|Default|SetAs%20Character _ascharacter))

(event EventTick
  (params (DeltaSeconds :type Float%20%28single-precision%29))
  (bind _as_character (Variables|Default|GetAs%20Character))
  (bind _charactermovement (Variables|/Script/Engine.Character|GetCharacterMovement _as_character))
  (if (AI|Components|NavMovement|IsFalling _charactermovement)
    (CallFunction|StopDrifting)
    (elif (Variables|Default|GetIsDrifting)
      (Variables|/Script/Engine.CharacterMovementComponent|SetGroundFriction _charactermovement 0.0)
      (Variables|/Script/Engine.MovementComponent|SetVelocity _charactermovement (* (Math|Vector|RotateVector (Transformation|GetActorForwardVector _as_character) (Math|Rotator|MakeRotator 0.0 0.0 (* (Variables|Default|GetCurrDriftAmount) -1.0 (Variables|Default|GetDriftDirection)))) (Math|Vector|VectorLength (Variables|/Script/Engine.MovementComponent|GetVelocity _charactermovement))))
      (Transformation|AddActorLocalRotation _as_character (Math|Rotator|MakeRotator 0.0 0.0 (* DeltaSeconds (CallFunction|GetDriftTurnRate) (Variables|Default|GetDriftDirection))) false false)
      (elif (Variables|Default|GetDriftInputHeld)
        (if (!= (Variables|Default|GetHorizontalInput) 0.0)
          (CallFunction|StartDrifting))))))

(fn StartDrifting
  (bind _as_character (Variables|Default|GetAs%20Character))
  (bind _horizontalinput (Variables|Default|GetHorizontalInput))
  (bind _returnvalue (Transformation|GetActorLocation _as_character))
  (Class|PlayerInterface|PlayDriftEffect(Message) (Components|GetOwner))
  (Variables|Default|SetIsDrifting true)
  (Transformation|SetActorRotation _as_character (Math|Interpolation|RInterpTo (Transformation|GetActorRotation _as_character) (Math|Rotator|FindLookatRotation _returnvalue (+ _returnvalue (Variables|/Script/Engine.MovementComponent|GetVelocity (Variables|/Script/Engine.Character|GetCharacterMovement _as_character)))) (Utilities|Time|GetWorldDeltaSeconds) 0.0))
  (if (> _horizontalinput 0.0)
    (Variables|Default|SetDriftDirection 1.0)
    (bind _askinzie_anim_bp (Utilities|Casting|CastToKinzieAnimBP (Components|SkeletalMesh|GetAnimInstance (Variables|/Script/Engine.Character|GetMesh _as_character)) :!label _label))
    (Variables|/Game/Rig/KinzieAnimBP.KinzieAnimBP_C|SetDrifting _askinzie_anim_bp true)
    (elif (< _horizontalinput 0.0)
      (Variables|Default|SetDriftDirection -1.0)
      (goto _label)
      (else
        (CallFunction|StopDrifting)))))

(fn StopDrifting
  (bind _as_character (Variables|Default|GetAs%20Character))
  (if (Variables|Default|GetIsDrifting)
    (Variables|Default|SetIsDrifting false)
    (Variables|/Script/Engine.CharacterMovementComponent|SetGroundFriction (Variables|/Script/Engine.Character|GetCharacterMovement _as_character) 1.0)
    (Class|PlayerInterface|StopDriftEffect(Message) _as_character)
    (bind _askinzie_anim_bp (Utilities|Casting|CastToKinzieAnimBP (Components|SkeletalMesh|GetAnimInstance (Variables|/Script/Engine.Character|GetMesh _as_character))))
    (Variables|/Game/Rig/KinzieAnimBP.KinzieAnimBP_C|SetDrifting _askinzie_anim_bp false)))

(fn GetDriftTurnRate
  (return (+ (Variables|Default|GetDriftTurnRate) (* (Variables|Default|GetHorizontalInput) (Variables|Default|GetDriftAdjustmentMax) (Variables|Default|GetDriftDirection)))))

(fn ActivateDriftInput
  (params (NewParam :type Boolean))
  (Variables|Default|SetDriftInputHeld NewParam))