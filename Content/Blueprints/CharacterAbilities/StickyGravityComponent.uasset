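; Scene component for a NinjaCharacter that provides speed-based sticky gravity by toggling the movement component's floor alignment.
; BeginPlay caches the owner as a NinjaCharacter.
; Each tick, floor alignment turns on above a high velocity threshold and off below a lower one, giving hysteresis between the two.
; A short line trace along the up vector also runs each tick but its result is unused, and gravity-alignment setters are left disconnected.
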(event EventBeginPlay
  (bind _asninja_character (Utilities|Casting|CastToNinjaCharacter (Components|GetOwner)))
  (Variables|Default|SetOwner _asninja_character))

(event EventTick
  (params (DeltaSeconds :type Float%20%28single-precision%29))
  (bind _returnvalue (Transformation|GetWorldLocation))
  (Collision|LineTraceByChannel _returnvalue (- _returnvalue (* (* (Math|Vector|GetUpVector) -1.0) 1e+02)) "TraceTypeQuery1" false 0 "None")
  (bind _asninja_character_movement_component (Utilities|Casting|CastToNinjaCharacterMovementComponent (Pawn|GetMovementComponent (Variables|Default|GetOwner))))
  (if (> (Math|Vector|VectorLength (Variables|/Script/Engine.MovementComponent|GetVelocity _asninja_character_movement_component)) 1.2e+03)
    (Variables|/Script/NinjaCharacter.NinjaCharacterMovementComponent|SetbAlignComponentToFloor _asninja_character_movement_component true)
    (elif (< (Math|Vector|VectorLength (Variables|/Script/Engine.MovementComponent|GetVelocity _asninja_character_movement_component)) 8e+02)
      (Variables|/Script/NinjaCharacter.NinjaCharacterMovementComponent|SetbAlignComponentToFloor _asninja_character_movement_component false))))