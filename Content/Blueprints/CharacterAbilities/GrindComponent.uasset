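; Character component that lets a skater grind along the spline of a GrindRail actor.
; StartGrinding snaps the owner to an interpolated closest distance and signs rail speed by velocity angle against the spline.
; Tick advances that distance, adjusts speed by slope and interpolates location and rotation, flipping facing for reverse travel.
; StopGrinding restores forward velocity and sets a re-grind timer, with toe sparks, sound and SkaterSkye_ABP's IsGrinding following grind state.
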(event Custom|TurnOnGrind
  (Variables|Default|SetCanGrind true))

(event Custom|TurnOnCanGrind
  (Variables|Default|SetCanGrind true))

(event Custom|TurnOn
  (Variables|Default|SetCanStopGrinding true))

(event EventBeginPlay
  (bind _ascharacter (Utilities|Casting|CastToCharacter (Components|GetOwner)))
  (Variables|Default|SetCharacterMovement (Variables|/Script/Engine.Character|GetCharacterMovement _ascharacter))
  (Variables|Default|SetMesh (Variables|/Script/Engine.Character|GetMesh _ascharacter))
  (bind _returnvalue (Niagara|SpawnSystemAttached "/Game/ParticlesFX/GrindSparksSystem.GrindSparksSystem" (Variables|Default|GetMesh) "DEF-toe_R" "0, 0,-0.200000" "0.000000,90.000000, 0" "KeepRelativeOffset" false))
  (bind _output_get (Variables|Default|SetRightGrindSparks _returnvalue))
  (bind _returnvalue_2 (Niagara|SpawnSystemAttached "/Game/ParticlesFX/GrindSparksSystem.GrindSparksSystem" (Variables|Default|GetMesh) "DEF-toe_L" "0, 0,-0.200000" "0.000000,90.000000, 0" "KeepRelativeOffset" false))
  (bind _output_get_2 (Variables|Default|SetLeftGrindSparks _returnvalue_2))
  (Components|Activation|Deactivate _output_get))

(event EventTick
  (params (DeltaSeconds :type Float%20%28single-precision%29))
  (CallFunction|GrindonRail))

(fn InitialRailPosition
  (bind _returnvalue (Components|GetOwner))
  (bind _grind_rail_reference (Variables|Default|GetGrind%20Rail%20Reference))
  (bind _returnvalue_2 (Transformation|GetActorLocation _returnvalue))
  (bind _spline (Variables|/Game/ThirdPersonCPP/GrindRail.GrindRail_C|GetSpline _grind_rail_reference))
  (bind _returnvalue_3 (Class|SplineComponent|FindInputKeyClosesttoWorldLocation _spline _returnvalue_2))
  (bind _returnvalue_4 (Math|Float|Truncate _returnvalue_3))
  (bind _returnvalue_5 (Spline|GetLocationatSplinePoint _spline _returnvalue_4 "World"))
  (bind _returnvalue_6 (+ _returnvalue_4 1))
  (return (Math|Float|Lerp (Spline|GetDistanceAlongSplineatSplinePoint _spline _returnvalue_4) (Spline|GetDistanceAlongSplineatSplinePoint _spline _returnvalue_6) (/ (Math|Vector|VectorLength (- (Spline|FindLocationClosesttoWorldLocation _spline (Transformation|GetActorLocation (Components|GetOwner)) "World") _returnvalue_5)) (Math|Vector|VectorLength (- (Spline|GetLocationatSplinePoint _spline _returnvalue_6 "World") _returnvalue_5))))))

(fn AdjustGrindSpeed
  (bind _raildelta (Variables|Default|GetRailDelta))
  (bind _grind_rail_reference (Variables|Default|GetGrind%20Rail%20Reference))
  (bind _returnvalue (- _raildelta 5.0))
  (bind _returnvalue_2 (- _raildelta 1e+02))
  (bind _spline (Variables|/Game/ThirdPersonCPP/GrindRail.GrindRail_C|GetSpline _grind_rail_reference))
  (bind _returnvalue_3 (Spline|GetLocationatDistanceAlongSpline _spline _returnvalue "World"))
  (bind _returnvalue_4 (Spline|GetLocationatDistanceAlongSpline _spline _returnvalue_2 "World"))
  (bind _z (Math|Vector|BreakVector _returnvalue_3))
  (bind _z_2 (Math|Vector|BreakVector _returnvalue_4))
  (bind _returnvalue_5 (- _z_2 _z))
  (Variables|Default|SetRailSpeed (+ (Variables|Default|GetRailSpeed) (Math|Float|Lerp (Math|Float|Lerp 0.0 (Math|Float|Lerp (Variables|Default|GetDecay) (* -1 (Variables|Default|GetSpeedGain)) (Math|Conversions|ToFloat(Boolean) (< (Variables|Default|GetRailSpeed) 0.0))) (Math|Float|MapRangeClamped _returnvalue_5 -9e+01 0.0 1.0 0.0)) (Math|Float|Lerp (Variables|Default|GetSpeedGain) (* -1 (Variables|Default|GetDecay)) (Math|Conversions|ToFloat(Boolean) (< (Variables|Default|GetRailSpeed) 0.0))) (Math|Float|MapRangeClamped _returnvalue_5 0.0 9e+01 0.0 1.0)))))

(fn GrindonRail
  (Utilities|IsValid (Variables|Default|GetGrind%20Rail%20Reference)
    (:Is%20Valid
      (bind _output_get (Variables|Default|SetRailDelta (+ (Variables|Default|GetRailDelta) (* (Variables|Default|GetRailSpeed) (Utilities|Time|GetWorldDeltaSeconds)))))
      (CallFunction|AdjustGrindSpeed)
      (Transformation|SetActorLocationAndRotation (Components|GetOwner) (Math|Interpolation|VInterpTo (Transformation|GetActorLocation (Components|GetOwner)) (+ (Spline|GetLocationatDistanceAlongSpline (Variables|/Game/ThirdPersonCPP/GrindRail.GrindRail_C|GetSpline (Variables|Default|GetGrind%20Rail%20Reference)) _output_get "World") (Math|Vector|MakeVector 0.0 0.0 1e+02)) (Utilities|Time|GetWorldDeltaSeconds) 0.0) (Math|Interpolation|RInterpTo (Transformation|GetActorRotation (Components|GetOwner)) (Math|Rotator|Lerp(Rotator) (Spline|GetRotationatDistanceAlongSpline (Variables|/Game/ThirdPersonCPP/GrindRail.GrindRail_C|GetSpline (Variables|Default|GetGrind%20Rail%20Reference)) (Variables|Default|GetRailDelta) "World") (Math|Rotator|CombineRotators (Math|Rotator|MakeRotator (* (.Roll (Math|Rotator|BreakRotator (Spline|GetRotationatDistanceAlongSpline (Variables|/Game/ThirdPersonCPP/GrindRail.GrindRail_C|GetSpline (Variables|Default|GetGrind%20Rail%20Reference)) (Variables|Default|GetRailDelta) "World"))) -1.0) (* (.Pitch (Math|Rotator|BreakRotator (Spline|GetRotationatDistanceAlongSpline (Variables|/Game/ThirdPersonCPP/GrindRail.GrindRail_C|GetSpline (Variables|Default|GetGrind%20Rail%20Reference)) (Variables|Default|GetRailDelta) "World"))) -1.0) (.Yaw (Math|Rotator|BreakRotator (Spline|GetRotationatDistanceAlongSpline (Variables|/Game/ThirdPersonCPP/GrindRail.GrindRail_C|GetSpline (Variables|Default|GetGrind%20Rail%20Reference)) (Variables|Default|GetRailDelta) "World")))) "0,180.000000, 0") (Math|Float|MapRangeClamped (Variables|Default|GetRailSpeed) -1e+01 1e+01 1.0 0.0)) (Utilities|Time|GetWorldDeltaSeconds) 0.0)) ; Interpolate player position/rotation for smoother attachment
      (Variables|/Script/Engine.MovementComponent|SetVelocity (Variables|Default|GetCharacterMovement) (Math|Conversions|ToVector(Float) (Variables|Default|GetRailSpeed)))
      (if (or (>= (Variables|Default|GetRailDelta) (Spline|GetSplineLength (Variables|/Game/ThirdPersonCPP/GrindRail.GrindRail_C|GetSpline (Variables|Default|GetGrind%20Rail%20Reference)))) (< (Variables|Default|GetRailDelta) 0.0))
        (CallFunction|StopGrinding)
        (Variables|Default|SetGrind%20Rail%20Reference 0)))))

(fn StopGrinding
  (Utilities|IsValid (Variables|Default|GetGrind%20Rail%20Reference)
    (:Is%20Valid
      (Variables|/Script/Engine.MovementComponent|SetVelocity (Variables|Default|GetCharacterMovement) (* (Transformation|GetActorForwardVector (Components|GetOwner)) (Math|Float|Absolute(Float) (Variables|Default|GetRailSpeed))))
      (Variables|Default|SetGrind%20Rail%20Reference 0)
      (Variables|Default|SetCangrind false)
      (bind _asskater_skye_abp (Utilities|Casting|CastToSkaterSkye_ABP (Components|SkeletalMesh|GetAnimInstance (Variables|Default|GetMesh))))
      (Variables|/Game/Skater_Skye/SkaterSkye_ABP.SkaterSkye_ABP_C|SetIsGrinding _asskater_skye_abp false)
      (Utilities|Time|SetTimerbyEvent (EventDispatchers|CreateEvent :!event Custom|TurnOnGrind) 0.25)
      (Audio|Components|Audio|Stop (Variables|Default|GetGrindSound))
      (Components|Activation|Deactivate (Variables|Default|GetRightGrindSparks)))))

(fn StartGrinding
  (params (OtherActor :type Actor%20Object%20Reference))
  (bind _railpos (CallFunction|InitialRailPosition))
  (Utilities|IsValid (Variables|Default|GetGrind%20Rail%20Reference)
    (:Is%20Not%20Valid
      (if (Variables|Default|GetCangrind)
        (bind _asgrind_rail (Utilities|Casting|CastToGrindRail OtherActor))
        (Utilities|IsValid (Variables|Default|GetGrind%20Rail%20Reference)
          (:Is%20Valid
            (bind _ascharacter (Utilities|Casting|CastToCharacter (Components|GetOwner)))
            (for _array_element (Class|PrimitiveComponent|GetOverlappingComponents (Variables|/Script/Engine.Character|GetCapsuleComponent _ascharacter))
              (if (Components|ComponentHasTag _array_element "RailEnd")
                (Utilities|IsValid (Variables|Default|GetGrind%20Rail%20Reference)
                  (:Is%20Valid
                    (CallFunction|StopGrinding)
                    (Variables|Default|SetGrind%20Rail%20Reference 0)
                    (Default|ResetBalance (Variables|Default|GetBalance))
                    (Variables|Default|SetCangrind false)
                    (Utilities|Time|SetTimerbyEvent (EventDispatchers|CreateEvent :!event Custom|TurnOnCanGrind) 0.1)
                    (bind _asskater_skye_abp (Utilities|Casting|CastToSkaterSkye_ABP (Components|SkeletalMesh|GetAnimInstance (Variables|Default|GetMesh))))
                    (Variables|/Game/Skater_Skye/SkaterSkye_ABP.SkaterSkye_ABP_C|SetIsGrinding _asskater_skye_abp false))))))
          (:Is%20Not%20Valid
            (Variables|Default|SetGrind%20Rail%20Reference _asgrind_rail)
            (Variables|Default|SetCanStopGrinding false)
            (Utilities|Time|SetTimerbyEvent (EventDispatchers|CreateEvent :!event Custom|TurnOn) 0.1)
            (bind _asskater_skye_abp_2 (Utilities|Casting|CastToSkaterSkye_ABP (Components|SkeletalMesh|GetAnimInstance (Variables|Default|GetMesh))))
            (Variables|/Game/Skater_Skye/SkaterSkye_ABP.SkaterSkye_ABP_C|SetIsGrinding _asskater_skye_abp_2 true)
            (Transformation|SetActorLocation (Components|GetOwner) (+ (Spline|GetLocationatDistanceAlongSpline (Variables|/Game/ThirdPersonCPP/GrindRail.GrindRail_C|GetSpline (Variables|Default|GetGrind%20Rail%20Reference)) _railpos "World") (Math|Vector|MakeVector 0.0 0.0 0.0)) false false)
            (Variables|Default|SetRailDelta _railpos)
            (CallFunction|GrindDirection)
            (Audio|PlaySoundatLocation "/Game/Sounds/FX/Character/MetalBracketHit_FSHOF_629.MetalBracketHit_FSHOF_629" (Transformation|GetActorLocation (Components|GetOwner)) "0, 0, 0" 1.0 1.0 0.0 0 0 0)
            (Components|Activation|Activate (Variables|Default|GetRightGrindSparks) false)
            (Audio|Components|Audio|Play (Variables|Default|GetGrindSound) 0.0)))))))

(fn GrindDirection
  (bind _charactermovement (Variables|Default|GetCharacterMovement))
  (bind _raildelta (Variables|Default|GetRailDelta))
  (bind _grind_rail_reference (Variables|Default|GetGrind%20Rail%20Reference))
  (bind _spline (Variables|/Game/ThirdPersonCPP/GrindRail.GrindRail_C|GetSpline _grind_rail_reference))
  (bind _velocity (Variables|/Script/Engine.MovementComponent|GetVelocity _charactermovement))
  (bind _returnvalue (Spline|GetRotationatDistanceAlongSpline _spline _raildelta "World"))
  (bind _returnvalue_2 (Math|Vector|RotateVector _velocity _returnvalue))
  (bind (_x _y _z) (Math|Vector|BreakVector _returnvalue_2))
  (Variables|Default|SetRailSpeed (* (Math|Vector|VectorLength (Math|Vector|MakeVector _x _y (/ _z 1.0))) (Math|Float|MapRangeClamped (CallFunction|CalculateAngleBetweenVectors _velocity (Spline|GetDirectionatDistanceAlongSpline _spline _raildelta "World")) 45.0 135.0 1.0 -1.0))))

(fn CalculateAngleBetweenVectors
  (params (v1 :type Vector) (v2 :type Vector))
  (return (Class|KismetMathLibrary|DegAcos (Math|Vector|DotProduct (Math|Vector|Normalize v1) (Math|Vector|Normalize v2)))))