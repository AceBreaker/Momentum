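; BrakeComponent is a character ability component that slows the owning Character's horizontal movement while its Braking flag is set.
; Each Tick it pulls CharacterMovement velocity toward zero on X and Y while keeping the current Z.
; Above a speed threshold it uses VInterpTo, and below it switches to a gentler lerp with delta time as alpha.
; The file does not set the Braking flag itself.
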(event EventBeginPlay)

(event EventTick
  (params (DeltaSeconds :type Float%20%28single-precision%29))
  (bind _returnvalue (Utilities|Time|GetWorldDeltaSeconds))
  (if (Variables|Default|GetBraking)
    (bind _ascharacter (Utilities|Casting|CastToCharacter (Components|GetOwner)))
    (if (> (Math|Vector|VectorLength (Variables|/Script/Engine.MovementComponent|GetVelocity (Variables|/Script/Engine.Character|GetCharacterMovement _ascharacter))) 2e+02)
      (Variables|/Script/Engine.MovementComponent|SetVelocity (Variables|/Script/Engine.Character|GetCharacterMovement _ascharacter) (Math|Interpolation|VInterpTo (Variables|/Script/Engine.MovementComponent|GetVelocity (Variables|/Script/Engine.Character|GetCharacterMovement _ascharacter)) (Math|Vector|MakeVector 0.0 0.0 (.Z (Math|Vector|BreakVector (Variables|/Script/Engine.MovementComponent|GetVelocity (Variables|/Script/Engine.Character|GetCharacterMovement _ascharacter))))) _returnvalue 5.0))
      (else
        (Variables|/Script/Engine.MovementComponent|SetVelocity (Variables|/Script/Engine.Character|GetCharacterMovement _ascharacter) (Math|Vector|Lerp(Vector) (Variables|/Script/Engine.MovementComponent|GetVelocity (Variables|/Script/Engine.Character|GetCharacterMovement _ascharacter)) (Math|Vector|MakeVector 0.0 0.0 (.Z (Math|Vector|BreakVector (Variables|/Script/Engine.MovementComponent|GetVelocity (Variables|/Script/Engine.Character|GetCharacterMovement _ascharacter))))) _returnvalue))))))