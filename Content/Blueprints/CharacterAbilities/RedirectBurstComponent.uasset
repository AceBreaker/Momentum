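; Character ability component that brakes momentum, then bursts the character along its facing direction, redirecting the speed it had before braking.
; SetBraking stores the current speed, starts the charge timer and Tick eases velocity toward zero; releasing early pauses the timer.
; When the timer fires, DoBurst applies the stored speed scaled by BurstDegradedPercent.
; Both functions toggle tagged charge/burst effects and the KinzieAnimBP Redirecting flag.
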(event EventBeginPlay)

(event EventTick
  (params (DeltaSeconds :type Float%20%28single-precision%29))
  (bind _returnvalue (Utilities|Time|GetWorldDeltaSeconds))
  (if (Variables|Default|GetBraking)
    (bind _ascharacter (Utilities|Casting|CastToCharacter (Components|GetOwner)))
    (if (> (Math|Vector|VectorLength (Variables|/Script/Engine.MovementComponent|GetVelocity (Variables|/Script/Engine.Character|GetCharacterMovement _ascharacter))) 2.5e+02)
      (Variables|/Script/Engine.MovementComponent|SetVelocity (Variables|/Script/Engine.Character|GetCharacterMovement _ascharacter) (Math|Interpolation|VInterpTo (Variables|/Script/Engine.MovementComponent|GetVelocity (Variables|/Script/Engine.Character|GetCharacterMovement _ascharacter)) "0, 0, 0" _returnvalue 5.0))
      (else
        (if (> (Math|Vector|VectorLength (Variables|/Script/Engine.MovementComponent|GetVelocity (Variables|/Script/Engine.Character|GetCharacterMovement _ascharacter))) 1e+02)
          _
          (else
            _))
        (Variables|/Script/Engine.MovementComponent|SetVelocity (Variables|/Script/Engine.Character|GetCharacterMovement _ascharacter) (Math|Vector|Lerp(Vector) (Variables|/Script/Engine.MovementComponent|GetVelocity (Variables|/Script/Engine.Character|GetCharacterMovement _ascharacter)) "0, 0, 0" _returnvalue))))))

(fn SetBraking
  (params (NewParam :type Boolean))
  (bind _returnvalue (Components|GetOwner))
  (bind _returnvalue_2 (Actor|GetComponentbyClass _returnvalue "/Script/Engine.CharacterMovementComponent"))
  (bind _returnvalue_3 (Actor|GetComponentsbyTag _returnvalue "/Script/Engine.ActorComponent" "ChargeEffect"))
  (bind _output (Utilities|Array|Get(acopy) _returnvalue_3))
  (bind _velocity (Variables|/Script/Engine.MovementComponent|GetVelocity _returnvalue_2))
  (bind _ascharacter (Utilities|Casting|CastToCharacter _returnvalue))
  (bind _output_get (Variables|Default|SetBraking NewParam))
  (if _output_get
    (Variables|Default|SetPrevVelLength (Math|Vector|VectorLength (Math|Vector|MakeVector (.x _velocity) (.y _velocity) (.z _velocity))))
    (bind _returnvalue_4 (Utilities|Time|SetTimerbyFunctionName self "DoBurst" (Variables|Default|GetBurstChargeTime)))
    (Variables|Default|SetBurstTimer _returnvalue_4)
    (bind _askinzie_anim_bp (Utilities|Casting|CastToKinzieAnimBP (Components|SkeletalMesh|GetAnimInstance (Variables|/Script/Engine.Character|GetMesh _ascharacter))))
    (Variables|/Game/Rig/KinzieAnimBP.KinzieAnimBP_C|SetRedirecting _askinzie_anim_bp true)
    (Components|Activation|Activate _output true)
    (else
      (Utilities|Time|PauseTimerbyHandle (Variables|Default|GetBurstTimer))
      (bind _askinzie_anim_bp_2 (Utilities|Casting|CastToKinzieAnimBP (Components|SkeletalMesh|GetAnimInstance (Variables|/Script/Engine.Character|GetMesh _ascharacter))))
      (Variables|/Game/Rig/KinzieAnimBP.KinzieAnimBP_C|SetRedirecting _askinzie_anim_bp_2 false)
      (Components|Activation|Deactivate _output))))

(fn DoBurst
  (bind _returnvalue (Components|GetOwner))
  (bind _ascharacter (Utilities|Casting|CastToCharacter _returnvalue))
  (Variables|/Script/Engine.MovementComponent|SetVelocity (Variables|/Script/Engine.Character|GetCharacterMovement _ascharacter) (* (* (Transformation|GetActorForwardVector _returnvalue) (Variables|Default|GetPrevVelLength)) (Variables|Default|GetBurstDegradedPercent)))
  (Variables|Default|SetBraking false)
  (Components|Activation|Activate (Utilities|Array|Get(acopy) (Actor|GetComponentsbyTag _ascharacter "/Script/Engine.ActorComponent" "BurstEffect")) true)
  (Components|Activation|Deactivate (Utilities|Array|Get(acopy) (Actor|GetComponentsbyTag _ascharacter "/Script/Engine.ActorComponent" "ChargeEffect")))
  (bind _askinzie_anim_bp (Utilities|Casting|CastToKinzieAnimBP (Components|SkeletalMesh|GetAnimInstance (Variables|/Script/Engine.Character|GetMesh _ascharacter))))
  (Variables|/Game/Rig/KinzieAnimBP.KinzieAnimBP_C|SetRedirecting _askinzie_anim_bp false))