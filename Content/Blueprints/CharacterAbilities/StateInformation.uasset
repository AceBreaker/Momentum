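; StateInformation is a character component that tracks whether its owning Character is grounded.
; On BeginPlay it casts and caches the owner as a Character.
; Each Tick it derives the grounded state from the movement component's falling check and triggers the owner-landed call on the transition from airborne to grounded.
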(event EventBeginPlay
  (bind _ascharacter (Utilities|Casting|CastToCharacter (Components|GetOwner)))
  (Variables|Default|SetOwnerReference _ascharacter))

(event EventTick
  (params (DeltaSeconds :type Float%20%28single-precision%29))
  (Variables|Default|SetPrevIsGrounded (Variables|Default|GetIsGrounded))
  (Variables|Default|SetIsGrounded (not (AI|Components|NavMovement|IsFalling (Pawn|GetMovementComponent (Variables|Default|GetOwnerReference)))))
  (if (and (Math|Boolean|NotEqual(Boolean) (Variables|Default|GetIsGrounded) (Variables|Default|GetPrevIsGrounded)) (Variables|Default|GetIsGrounded))
    (Default|CallOnOwnerLanded)))