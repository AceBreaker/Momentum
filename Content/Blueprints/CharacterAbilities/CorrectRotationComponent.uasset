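; Actor component that gradually levels the skater character's rotation while airborne.
; On begin play it caches its owning Character, then each tick checks that it is a SkaterSkyeCharacter_BP that is falling and not in a ledge stall.
; When so, it uses RInterpTo to ease pitch and roll back to zero while keeping the current yaw.
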(event EventBeginPlay
  (bind _ascharacter (Utilities|Casting|CastToCharacter (Components|GetOwner)))
  (Variables|Default|SetOwner _ascharacter))

(event EventTick
  (params (DeltaSeconds :type Float%20%28single-precision%29))
  (CallFunction|CorrectRotation))

(fn CorrectRotation
  (bind _owner (Variables|Default|GetOwner))
  (bind _returnvalue (Transformation|GetActorRotation _owner))
  (bind _asskater_skye_character_bp (Utilities|Casting|CastToSkaterSkyeCharacter_BP (Variables|Default|GetOwner)))
  (if (and (AI|Components|NavMovement|IsFalling (Pawn|GetMovementComponent _owner)) (not (Variables|/Game/Skater_Skye/SkaterSkyeCharacter_BP.SkaterSkyeCharacter_BP_C|GetLedgeStall _asskater_skye_character_bp)))
    (Transformation|SetActorRotation _owner (Math|Interpolation|RInterpTo _returnvalue (Math|Rotator|MakeRotator 0.0 0.0 (.Yaw (Math|Rotator|BreakRotator _returnvalue))) (Utilities|Time|GetWorldDeltaSeconds) 1.0))))