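; Skater character component that catches surfaces and redirects momentum off edges, using a one-second readiness window that also enables grind collision.
; When armed airborne, a hit pulls the skater into the surface; this and qualifying downward hits briefly align gravity to the normal, then shake the camera.
; When armed grounded, starting to fall stalls the skater, turns them toward their previous down vector, then relaunches at saved speed and re-arms.
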(event Custom|SetReadyToCatch
  (params (Character :type Skater%20Skye%20Character%20BP%20Object%20Reference))
  (Utilities|Time|SetTimerbyEvent (delegate Custom|Unready) 1.0)
  (if (Variables|Default|GetFalling)
    (Variables|Default|SetReadyToCatch true)
    (else
      (Variables|Default|SetReadyToRedirect true)))
  (Collision|SetCollisionEnabled (Variables|/Game/Skater_Skye/SkaterSkyeCharacter_BP.SkaterSkyeCharacter_BP_C|GetGrindCollider Character) "QueryAndPhysics"))

(event Custom|Unready
  (CallFunction|UnreadyFunction (stale Custom|SetReadyToCatch Character)))

(event Custom|Hit
  (params (NewParam :type Vector) (NewParam2 :type Ninja%20Character%20Movement%20Component%20Object%20Reference))
  (bind _returnvalue (* NewParam -1.0))
  (bind _returnvalue_2 (Math|Vector|VectorUp))
  (bind _returnvalue_3 (Math|Vector|DotProduct NewParam _returnvalue_2))
  (if (or (Variables|Default|GetReadyToCatch) (and (> (Math|Vector|DotProduct (Variables|/Script/Engine.MovementComponent|GetVelocity NewParam2) (* _returnvalue_2 -1.0)) 0.0) (or (> _returnvalue_3 0.1) (< _returnvalue_3 -0.1))))
    (if (Variables|Default|GetReadyToCatch)
      (Variables|/Script/Engine.MovementComponent|SetVelocity NewParam2 (+ (Variables|/Script/Engine.MovementComponent|GetVelocity NewParam2) (* _returnvalue 1e+04))))
    (Variables|Default|SetReadyToCatch false)
    (Variables|/Script/NinjaCharacter.NinjaCharacterMovementComponent|SetbAlignComponentToGravity NewParam2 true)
    (Class|NinjaCharacterMovementComponent|SetFixedGravityDirection NewParam2 _returnvalue)
    (Utilities|FlowControl|Delay 0.1)
    (Variables|/Script/NinjaCharacter.NinjaCharacterMovementComponent|SetbAlignComponentToGravity NewParam2 false)
    (Class|NinjaCharacterMovementComponent|SetFixedGravityDirection NewParam2 (Math|Vector|MakeVector 0.0 0.0 -1.0))
    (CameraShakes|StartCameraShake (Game|GetPlayerCameraManager 0) "/Game/LandingScreenShake.LandingScreenShake_C" 1.0 "CameraLocal" "0, 0, 0")))

(event Custom|Launch
  (bind _returnvalue (Components|GetOwner))
  (Variables|/Script/Engine.MovementComponent|SetVelocity (Pawn|GetMovementComponent (stale EventTick _asskater_skye_character_bp)) (* (Math|Vector|Normalize (Math|Vector|Lerp(Vector) (Transformation|GetActorForwardVector _returnvalue) (* (Transformation|GetActorUpVector _returnvalue) -1.0) 0.25)) (Variables|Default|GetNewSpeed)))
  (Utilities|Time|InvalidateTimerHandle (Variables|Default|GetRedirectTime))
  (Variables|/Game/Skater_Skye/SkaterSkyeCharacter_BP.SkaterSkyeCharacter_BP_C|SetLedgeStall (stale EventTick _asskater_skye_character_bp) false)
  (CallFunction|SetReadytoCatch (stale EventTick _asskater_skye_character_bp))
  (Variables|Default|SetReadyToRedirect false)
  (Variables|/Game/HandleAutoManualCamera.HandleAutoManualCamera_C|SetCameraRotationOveridden (Variables|/Game/Skater_Skye/SkaterSkyeCharacter_BP.SkaterSkyeCharacter_BP_C|GetHandleAutoManualCamera (stale EventTick _asskater_skye_character_bp)) false))

(event Custom|UnreadyCharacter
  (params (Character :type Skater%20Skye%20Character%20BP%20Object%20Reference))
  (CallFunction|UnreadyFunction Character))

(event Custom|UnreadyFunction
  (params (Character :type Skater%20Skye%20Character%20BP%20Object%20Reference))
  (Variables|Default|SetReadyToCatch false)
  (Collision|SetCollisionEnabled (Variables|/Game/Skater_Skye/SkaterSkyeCharacter_BP.SkaterSkyeCharacter_BP_C|GetGrindCollider Character) "NoCollision")
  (Variables|Default|SetReadyToRedirect false))

(event EventTick
  (params (DeltaSeconds :type Float%20%28single-precision%29))
  (bind _returnvalue (Components|GetOwner))
  (bind _returnvalue_2 (Components|GetOwner))
  (bind _returnvalue_3 (Components|GetOwner))
  (bind _returnvalue_4 (Transformation|GetActorLocation _returnvalue_2))
  (bind _asskater_skye_character_bp (Utilities|Casting|CastToSkaterSkyeCharacter_BP _returnvalue_3))
  (if (Utilities|Time|IsValidTimerHandle (Variables|Default|GetRedirectTime))
    (Variables|/Script/Engine.MovementComponent|SetVelocity (Pawn|GetMovementComponent _asskater_skye_character_bp) "0, 0, 0")
    (Variables|/Script/Engine.SpringArmComponent|SetCameraRotationLagSpeed (Variables|/NinjaCharacter/NinjaCharacter/Blueprints/NinjaPlayerCharacter_BP.NinjaPlayerCharacter_BP_C|GetCameraBoom _asskater_skye_character_bp) 0.0)
    (else
      (if (Math|Boolean|ANDBoolean (AI|Components|NavMovement|IsFalling (Pawn|GetMovementComponent _asskater_skye_character_bp)) (not (Variables|Default|GetFalling)) (Variables|Default|GetReadyToRedirect) (not (Utilities|Time|IsValidTimerHandle (Variables|Default|GetRedirectTime))))
        (Variables|Default|SetNewDirection (Variables|Default|GetPreviousDownVector))
        (Variables|Default|SetNewSpeed (Math|Vector|VectorLength (Variables|/Script/Engine.MovementComponent|GetVelocity (Pawn|GetMovementComponent _asskater_skye_character_bp))))
        (Variables|/Game/Skater_Skye/SkaterSkyeCharacter_BP.SkaterSkyeCharacter_BP_C|SetLedgeStall _asskater_skye_character_bp true)
        (bind _returnvalue_5 (Utilities|Time|SetTimerbyEvent (delegate Custom|Launch) 0.5))
        (Variables|Default|SetRedirectTime _returnvalue_5)
        (Transformation|SetActorRotation _returnvalue_2 (Math|Rotator|FindLookatRotation _returnvalue_4 (+ _returnvalue_4 (* (Math|Vector|Lerp(Vector) (Variables|Default|GetNewDirection) (Transformation|GetActorForwardVector _returnvalue_2) 0.1) 1e+03))) true)
        (Variables|/Script/Engine.SpringArmComponent|SetCameraRotationLagSpeed (Variables|/NinjaCharacter/NinjaCharacter/Blueprints/NinjaPlayerCharacter_BP.NinjaPlayerCharacter_BP_C|GetCameraBoom _asskater_skye_character_bp) 0.0)
        (Variables|/Game/HandleAutoManualCamera.HandleAutoManualCamera_C|SetCameraRotationOveridden (Variables|/Game/Skater_Skye/SkaterSkyeCharacter_BP.SkaterSkyeCharacter_BP_C|GetHandleAutoManualCamera _asskater_skye_character_bp) true)
        (Transformation|SetActorLocation _returnvalue (+ (Transformation|GetActorLocation _returnvalue) (* (Math|Vector|Normalize (Variables|/Script/Engine.MovementComponent|GetVelocity (Pawn|GetMovementComponent _asskater_skye_character_bp))) 5e+01)) false false))
      (Variables|Default|SetFalling (AI|Components|NavMovement|IsFalling (Pawn|GetMovementComponent _asskater_skye_character_bp)))
      (Variables|Default|SetPreviousDownVector (* (Transformation|GetActorUpVector _returnvalue_3) -1.0)))))

(fn NewFunction0)