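; Character component that makes jumping forgiving, with input buffering, coyote time and variable jump height.
; Tick advances both timers, refreshed by AttemptToJump and the owner's can-jump interface, then fires a normal or sideways grind-rail jump when both windows overlap.
; Jumps add force along actor up, with smoke and dispatcher-driven sound.
; Releasing cuts upward velocity proportionally to speed, while Ninja movement gravity scale switches on airborne Held state.
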(event Custom|AttemptToJump
  (Variables|Default|SetBufferTime 0.0))

(event Custom|ReleaseJump
  (bind _as_character (Variables|Default|GetAs%20Character))
  (bind _charactermovement (Variables|/Script/Engine.Character|GetCharacterMovement _as_character))
  (if (and (AI|Components|NavMovement|IsFalling _charactermovement) (> (.z (Variables|/Script/Engine.MovementComponent|GetVelocity _charactermovement)) 0.0))
    (Variables|/Script/Engine.MovementComponent|SetVelocity _charactermovement (Math|Vector|MakeVector (.x (Variables|/Script/Engine.MovementComponent|GetVelocity _charactermovement)) (.y (Variables|/Script/Engine.MovementComponent|GetVelocity _charactermovement)) (* (.z (Variables|/Script/Engine.MovementComponent|GetVelocity _charactermovement)) (Math|Float|Clamp(Float) (Math|Float|Lerp 0.2 0.8 (- 1.0 (/ (.z (Variables|/Script/Engine.MovementComponent|GetVelocity _charactermovement)) 1e+03))) 0.2 0.8))))))

(event Custom|PlaySound
  (Audio|PlaySoundatLocation (Variables|Default|GetSoundToPlay) (Transformation|GetActorLocation (Components|GetOwner)) "0, 0, 0" 1.0 1.0 0.0 0 0 0))

(event EventBeginPlay
  (EventDispatchers|BindEventtoJumpDispatcher (delegate Custom|PlaySound))
  (bind _ascharacter (Utilities|Casting|CastToCharacter (Components|GetOwner)))
  (Variables|Default|SetAs%20Character _ascharacter))

(event EventTick
  (params (DeltaSeconds :type Float%20%28single-precision%29))
  (CallFunction|UpdateGravityStrength)
  (Variables|Default|SetBufferTime (+ (Variables|Default|GetBufferTime) DeltaSeconds))
  (Variables|Default|SetCoyoteTime (+ (Variables|Default|GetCoyoteTime) DeltaSeconds))
  (bind _ascharacter (Utilities|Casting|CastToCharacter (Components|GetOwner)))
  (bind _yes (Class|CanJump|ICanJump(Message) (Components|GetOwner)))
  (if (not _yes)
    _
    (else
      (Variables|Default|SetCoyoteTime 0.0)))
  (if (CallFunction|CanJump)
    (bind _ascharacter_2 (Utilities|Casting|CastToCharacter (Components|GetOwner)))
    (bind (_canjump _helddirection) (Class|CanJump|ICanJumpfromRail(Message) _ascharacter_2))
    (Default|CallPreparetoJump)
    (if _canjump
      (CallFunction|ExecuteGrindRailJump _helddirection)
      (else
        (CallFunction|ExecuteJump)))))

(fn ExecuteJump
  (bind _returnvalue (Components|GetOwner))
  (bind _as_character (Variables|Default|GetAs%20Character))
  (bind _charactermovement (Variables|/Script/Engine.Character|GetCharacterMovement _as_character))
  (Character|Jump _as_character)
  (if (Math|Boolean|ANDBoolean (< (.z (Variables|/Script/Engine.MovementComponent|GetVelocity _charactermovement)) 0.0) true (CallFunction|ResetVert))
    (Variables|/Script/Engine.MovementComponent|SetVelocity _charactermovement (Math|Vector|MakeVector (.x (Variables|/Script/Engine.MovementComponent|GetVelocity _charactermovement)) (.y (Variables|/Script/Engine.MovementComponent|GetVelocity _charactermovement)) (select (> (Math|Vector|DotProduct (Variables|/Script/Engine.MovementComponent|GetVelocity _charactermovement) (Math|Vector|VectorDown)) 0.5) (.z (Variables|/Script/Engine.MovementComponent|GetVelocity _charactermovement)) 0.0))))
  (Variables|/Script/Engine.MovementComponent|SetVelocity _charactermovement (+ (Variables|/Script/Engine.MovementComponent|GetVelocity _charactermovement) (* (Transformation|GetActorUpVector _as_character) (Variables|Default|GetJumpForce))))
  (Variables|Default|SetCoyoteTime (Variables|Default|GetAvailableCoyoteTime))
  (Variables|Default|SetBufferTime (Variables|Default|GetAvailableBufferTime))
  (Default|CallJumpDispatcher)
  (Niagara|SpawnSystematLocation "/Game/ParticlesFX/LandingSmoke.LandingSmoke" (- (Transformation|GetActorLocation _returnvalue) (* (Transformation|GetActorUpVector _returnvalue) 96.0)) (Transformation|GetActorRotation _returnvalue)))

(fn CanJump
  (bind _returnvalue (Components|GetOwner))
  (Utilities|Casting|CastToCharacter _returnvalue)
  (Class|CanJump|ICanJump(Message) _returnvalue)
  (return (Math|Boolean|ANDBoolean (< (Variables|Default|GetBufferTime) (Variables|Default|GetAvailableBufferTime)) (< (Variables|Default|GetCoyoteTime) (Variables|Default|GetAvailableCoyoteTime)) true)))

(fn UpdateGravityStrength
  (bind _as_character (Variables|Default|GetAs%20Character))
  (bind _returnvalue (Pawn|GetMovementComponent _as_character))
  (bind _asninja_character_movement_component (Utilities|Casting|CastToNinjaCharacterMovementComponent _returnvalue))
  (if (and (AI|Components|NavMovement|IsFalling _returnvalue) (Variables|Default|GetHeld))
    (Variables|/Script/Engine.CharacterMovementComponent|SetGravityScale _asninja_character_movement_component (Variables|Default|GetUpwardGravity))
    (else
      (Variables|/Script/Engine.CharacterMovementComponent|SetGravityScale _asninja_character_movement_component (Variables|Default|GetDownwardGravity)))))

(fn DebugPrint)

(fn ResetVert
  (bind _returnvalue (Components|GetOwner))
  (Utilities|Casting|CastToCharacter _returnvalue)
  (bind _yes (Class|CanJump|ICanJump(Message) _returnvalue))
  (return (or _yes (< (Variables|Default|GetCoyoteTime) (Variables|Default|GetAvailableCoyoteTime)))))

(fn ExecuteGrindRailJump
  (params (HeldDir :type Vector))
  (bind _returnvalue (Components|GetOwner))
  (bind _ascharacter (Utilities|Casting|CastToCharacter _returnvalue))
  (Character|Jump _ascharacter)
  (if (Math|Boolean|ANDBoolean (< (.z (Variables|/Script/Engine.MovementComponent|GetVelocity (Variables|/Script/Engine.Character|GetCharacterMovement _ascharacter))) 0.0) true (CallFunction|ResetVert))
    (Variables|/Script/Engine.MovementComponent|SetVelocity (Variables|/Script/Engine.Character|GetCharacterMovement _ascharacter) (Math|Vector|MakeVector (+ (.x (Variables|/Script/Engine.MovementComponent|GetVelocity (Variables|/Script/Engine.Character|GetCharacterMovement _ascharacter))) (.X (Math|Vector|BreakVector (* (Math|Vector|VectorGetAbs (Transformation|GetActorRightVector _ascharacter)) (* HeldDir 1e+03))))) (+ (.y (Variables|/Script/Engine.MovementComponent|GetVelocity (Variables|/Script/Engine.Character|GetCharacterMovement _ascharacter))) (.Y (Math|Vector|BreakVector (* (Math|Vector|VectorGetAbs (Transformation|GetActorRightVector _ascharacter)) (* HeldDir 1e+03))))) 0.0)))
  (Variables|/Script/Engine.MovementComponent|SetVelocity (Variables|/Script/Engine.Character|GetCharacterMovement _ascharacter) (+ (Variables|/Script/Engine.MovementComponent|GetVelocity (Variables|/Script/Engine.Character|GetCharacterMovement _ascharacter)) (* (Transformation|GetActorUpVector _ascharacter) (Variables|Default|GetJumpForce)) (* (Math|Vector|VectorGetAbs (Transformation|GetActorRightVector _ascharacter)) (* HeldDir 1e+03))))
  (Variables|Default|SetCoyoteTime (Variables|Default|GetAvailableCoyoteTime))
  (Variables|Default|SetBufferTime (Variables|Default|GetAvailableBufferTime))
  (Default|CallJumpDispatcher)
  (Niagara|SpawnSystematLocation "/Game/ParticlesFX/LandingSmoke.LandingSmoke" (- (Transformation|GetActorLocation _returnvalue) (* (Transformation|GetActorUpVector _returnvalue) 96.0)) (Transformation|GetActorRotation _returnvalue)))