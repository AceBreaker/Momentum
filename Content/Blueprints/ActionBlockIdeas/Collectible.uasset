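; Spinning collectible for the skater game that awards score, or one of the S-K-Y-E letters when Letter is set, which also swaps its mesh.
; On BeginPlay it registers with the CollectibleManager, binds to the player's level-restart dispatcher and tints its mesh and light a random color.
; Overlap by an actor with a Collector component plays tinted effects, hides it and updates the manager.
; EnableCollectible restores collected items and subtracts their points.
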(event Custom|EnableCollectible
  (if (Variables|Default|GetIsCollected)
    (Rendering|SetActorHiddenInGame false)
    (Collision|SetCollisionEnabled (Variables|Default|GetSphere) "QueryAndPhysics")
    (Default|CallCollectibleReenabled)
    (Default|UpdateScore (Variables|Default|GetCoinsCounter) (* (Variables|Default|GetScorePoints) -1))
    (Variables|Default|SetIsCollected false)))

(event EventBeginPlay
  (bind _staticmesh (Variables|Default|GetStaticMesh))
  (bind _outactors (Actor|GetAllActorswithTag "CoinsManager"))
  (bind _ascollectible_manager (Utilities|Casting|CastToCollectibleManager (Utilities|Array|Get(acopy) _outactors)))
  (bind _output_get (Variables|Default|SetCoinsCounter _ascollectible_manager))
  (Default|AddCoin _output_get)
  (bind _returnvalue (Rendering|Material|CreateDynamicMaterialInstance _staticmesh 0 (Rendering|Material|GetMaterial _staticmesh 0) "PaintColor" :!class /Script/Engine.PrimitiveComponent))
  (bind _output_get_2 (Variables|Default|SetColor (Math|Color|MakeColor (Math|Conversions|ToFloat(Integer) (Math|Random|RandomInteger 2)) (Math|Conversions|ToFloat(Integer) (Math|Random|RandomInteger 2)) (Math|Conversions|ToFloat(Integer) (Math|Random|RandomInteger 2)))))
  (Rendering|Material|SetVectorParameterValue _returnvalue "PaintColor" _output_get_2 :!class /Script/Engine.MaterialInstanceDynamic)
  (Rendering|Components|Light|SetLightColor (Variables|Default|GetPointLight) _output_get_2 true)
  (bind _asskater_skye_character_bp (Utilities|Casting|CastToSkaterSkyeCharacter_BP (Game|Player|GetPlayerPawn 0)))
  (EventDispatchers|BindEventtoRestartLevelDispatcher _asskater_skye_character_bp (EventDispatchers|CreateEvent :!event Custom|EnableCollectible)))

(event Collision|EventActorBeginOverlap
  (params (OtherActor :type Actor%20Object%20Reference))
  (bind _returnvalue (Transformation|GetActorLocation))
  (bind _coinscounter (Variables|Default|GetCoinsCounter))
  (Utilities|IsValid (Actor|GetComponentbyClass OtherActor "/Game/Collector.Collector_C")
    (:Is%20Valid
      (Audio|SpawnSoundatLocation (Variables|Default|GetCollectAudio) _returnvalue "0, 0, 0" 1.0 1.0 0.0 0 0)
      (bind _returnvalue_2 (Niagara|SpawnSystematLocation (Variables|Default|GetCollectParticle) _returnvalue))
      (Effects|Components|ParticleSystem|SetVectorParameter _returnvalue_2 "PaintColor" (Math|Conversions|ToVector(LinearColor) (Variables|Default|GetColor)))
      (Default|CallGrabbedCollectible)
      (Rendering|SetActorHiddenInGame true)
      (Collision|SetCollisionEnabled (Variables|Default|GetSphere) "NoCollision")
      (Variables|Default|SetIsCollected true)
      (if (Utilities|Enum|Equal(Enum) (Variables|Default|GetLetter) "NewEnumerator4")
        (Default|UpdateScore _coinscounter (Variables|Default|GetScorePoints))
        (else
          (Default|UpdateSKYELetters _coinscounter (Variables|Default|GetLetter) true))))))

(event EventTick
  (params (DeltaSeconds :type Float%20%28single-precision%29))
  (Transformation|AddActorLocalRotation "0,0.900000, 0" false false))

(fn ConstructionScript
  (bind _letter (Variables|Default|GetLetter))
  (bind _staticmesh (Variables|Default|GetStaticMesh))
  (if (not (Utilities|Enum|Equal(Enum) _letter "NewEnumerator4"))
    (Components|StaticMesh|SetStaticMesh _staticmesh (Utilities|Select :Index _letter :NewEnumerator0 "/Game/Models/CollectLettersS.CollectLettersS" :NewEnumerator1 "/Game/Models/CollectLettersK.CollectLettersK" :NewEnumerator2 "/Game/Models/CollectLettersY.CollectLettersY" :NewEnumerator3 "/Game/Models/CollectLettersE.CollectLettersE" :NewEnumerator4 "/Game/Models/MajorActors/SprayPaintCan.SprayPaintCan"))
    (Transformation|SetWorldScale3D _staticmesh "1.000000,1.000000,1.000000")
    (Rendering|Material|SetMaterial _staticmesh 0 "/Game/Models/Material_001.Material_001")
    (Utilities|Array|Add (Variables|Actor|GetTags) "Hidden")))

(fn PrintScore
  (Development|PrintString (Utilities|String|Append (Utilities|String|MakeLiteralString "CurrentScore: ") (Utilities|String|ToString(Integer) (Variables|Default|GetScorePoints)))))