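; Actor component that computes slope-based speed and acceleration multipliers for its owner, which it expects to be a Character.
; Each tick it traces down from the owner and dots the surface normal with horizontal forward, feeding SpeedCurve into Mul and AccelCurve into AMul.
; When the hit normal is horizontal, Mul instead samples SpeedCurve with the negated vertical component of velocity direction.
; Nothing here applies the multipliers, and GetMultiplier is a stub returning zero.
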(event EventBeginPlay
  (bind _output_get (Variables|Default|SetOwner (Components|GetOwner)))
  (bind _ascharacter (Utilities|Casting|CastToCharacter _output_get))
  (Variables|Default|SetOwnerAsCharacter _ascharacter))

(event EventTick
  (params (DeltaSeconds :type Float%20%28single-precision%29))
  (bind _owner (Variables|Default|GetOwner))
  (bind _owner_2 (Variables|Default|GetOwner))
  (bind _returnvalue (Transformation|GetActorLocation _owner))
  (bind _returnvalue_2 (Transformation|GetActorForwardVector _owner_2))
  (bind (_x _y) (Math|Vector|BreakVector _returnvalue_2))
  (bind (_outhit _returnvalue_3) (Collision|LineTraceByChannel _returnvalue (+ _returnvalue (* (* (Transformation|GetActorUpVector _owner) -1.0) 1.1e+02)) "TraceTypeQuery2" false 0 "None"))
  (Variables|Default|SetAMul (Math|Curves|GetFloatValue (Variables|Default|GetAccelCurve) (Math|Vector|DotProduct (.ImpactNormal (Collision|BreakHitResult _outhit)) (Math|Vector|Normalize (Math|Vector|MakeVector _x _y 0.0)))))
  (Variables|Default|SetMul (Math|Curves|GetFloatValue (Variables|Default|GetSpeedCurve) (Math|Vector|DotProduct (.ImpactNormal (Collision|BreakHitResult _outhit)) (Math|Vector|Normalize (Math|Vector|MakeVector _x _y 0.0)))))
  (if (and (Math|Float|NearlyEqual(Float) (.Z (Math|Vector|BreakVector (.ImpactNormal (Collision|BreakHitResult _outhit)))) 0.0 0.0001) _returnvalue_3)
    (if (Math|Vector|NotEqual(Vector) (.ImpactNormal (Collision|BreakHitResult _outhit)) (Math|Vector|VectorUp) 0.0001)
      (bind _output_get (Variables|Default|SetMul (Math|Curves|GetFloatValue (Variables|Default|GetSpeedCurve) (* -1 (Math|Vector|DotProduct (Math|Vector|Normalize (Transformation|GetVelocity (Variables|Default|GetOwner))) (Math|Vector|VectorUp)))))))))

(fn GetMultiplier
  (return 0.0))