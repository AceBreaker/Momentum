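; SkinData is a skater character customization Blueprint that recolors skeletal mesh parts such as hair, body, clothing, skates and accessories.
; SetSelectedMesh maps a part enum to its component, and SetColor feeds it to SetMeshColor, which records mesh and color in a map.
; Gender-specific index maps pick material slots for dynamic instances, with negative indices tinting all slots.
; SaveSkin and LoadSkin are empty stubs.
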(event EventBeginPlay)

(fn ConstructionScript)

(fn SetSkeletalMesh
  (params (MeshToChange :type Skinned%20Mesh%20Component%20Object%20Reference) (NewMesh :type Skeletal%20Mesh%20Object%20Reference))
  (Class|SkinnedMeshComponent|SetSkeletalMesh MeshToChange NewMesh true))

(fn SaveSkin)

(fn LoadSkin)

(fn SetMeshColor
  (params (MeshToChange :type Skinned%20Mesh%20Component%20Object%20Reference) (NewParam1 :type Linear%20Color%20Structure) (MeshEnum :type CharacterParts%20Enum :default "NewEnumerator0"))
  (bind _output_get (Variables|Default|SetMeshEnum MeshEnum))
  (Utilities|Map|Add (Variables|Default|GetDatas) _output_get (Utilities|Struct|MakeCharacterPartData (Variables|/Script/Engine.SkinnedMeshComponent|GetSkeletalMesh MeshToChange) NewParam1))
  (if (Variables|Default|GetIsMale)
    (if (.ReturnValue (Utilities|Map|Find (Variables|Default|GetMaleIndicies) (Variables|Default|GetMeshEnum)))
      (CallFunction|SetGenderedColors MeshToChange NewParam1 (.Value (Utilities|Map|Find (Variables|Default|GetMaleIndicies) (Variables|Default|GetMeshEnum))))
      (else
        (CallFunction|SetGenderedColors MeshToChange NewParam1)))
    (elif (.ReturnValue (Utilities|Map|Find (Variables|Default|GetFemaleIndices) (Variables|Default|GetMeshEnum)))
      (CallFunction|SetGenderedColors MeshToChange NewParam1 (.Value (Utilities|Map|Find (Variables|Default|GetFemaleIndices) (Variables|Default|GetMeshEnum))))
      (CallFunction|SetGenderedColors MeshToChange NewParam1)
      (else
        (CallFunction|SetGenderedColors MeshToChange NewParam1)))))

(fn SetGender
  (params (NewParam :type Boolean))
  (Variables|Default|SetIsMale NewParam))

(fn SetGenderedColors
  (params (MeshToChange :type Skinned%20Mesh%20Component%20Object%20Reference) (NewParam1 :type Linear%20Color%20Structure) (MaterialIndex :type Integer))
  (if (>= MaterialIndex 0)
    (bind _returnvalue (Rendering|Material|CreateDynamicMaterialInstance MeshToChange MaterialIndex (Rendering|Material|GetMaterial MeshToChange MaterialIndex) "None" :!class /Script/Engine.PrimitiveComponent))
    (Rendering|Material|SetVectorParameterValue _returnvalue "Param" NewParam1 :!class /Script/Engine.MaterialInstanceDynamic)
    (else
      (for (_array_element _array_index) (Rendering|Material|GetMaterials MeshToChange)
        (bind _returnvalue_2 (Rendering|Material|CreateDynamicMaterialInstance MeshToChange _array_index _array_element "None" :!class /Script/Engine.PrimitiveComponent))
        (Rendering|Material|SetVectorParameterValue _returnvalue_2 "Param" NewParam1 :!class /Script/Engine.MaterialInstanceDynamic)))))

(fn SetColor
  (params (NewColor :type Linear%20Color%20Structure))
  (CallFunction|SetMeshColor (Variables|Default|GetSelectedSkeletalMesh) NewColor (Variables|Default|GetMeshEnum)))

(fn SetSelectedMesh
  (params (NewParam :type CharacterParts%20Enum :default "NewEnumerator0"))
  (Variables|Default|SetMeshEnum NewParam)
  (Variables|Default|SetSelectedSkeletalMesh (Utilities|Select :Index NewParam :NewEnumerator0 (Variables|Default|GetHair) :NewEnumerator1 (Variables|Default|GetBody) :NewEnumerator2 (Variables|Default|GetTop) :NewEnumerator3 (Variables|Default|GetBottom) :NewEnumerator4 (Variables|Default|GetSkates) :NewEnumerator5 (Variables|Default|GetGlasses) :NewEnumerator6 (Variables|Default|GetHeadphones) :NewEnumerator7 (Variables|Default|GetBody) :NewEnumerator8 0)))