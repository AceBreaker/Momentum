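; SkinManager restores a saved character skin on the player, using the slot named in MomentumGameInstance and reporting success back to it.
; LoadSkin reads the CharacterSave and, for each part, resolves the component through GetMeshesMessage, then swaps its skeletal mesh and applies its color.
; Colors set "Param" on dynamic material instances, with slots chosen from male or female index maps; a negative index recolors every slot.
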(event Custom|RequestLoadSkin
  (bind _asmomentum_game_instance (Utilities|Casting|CastToMomentumGameInstance (Game|GetGameInstance)))
  (bind _success (CallFunction|LoadSkin (Variables|/Game/MomentumGameInstance.MomentumGameInstance_C|GetSkinToLoad _asmomentum_game_instance)))
  (Variables|/Game/MomentumGameInstance.MomentumGameInstance_C|SetSkinLoaded _asmomentum_game_instance _success))

(event EventBeginPlay)

(event Collision|EventActorBeginOverlap
  (params (OtherActor :type Actor%20Object%20Reference)))

(event EventTick
  (params (DeltaSeconds :type Float%20%28single-precision%29)))

(fn ConstructionScript)

(fn LoadSkin
  (params (Filename :type String))
  (bind _returnvalue (SaveGame|LoadGamefromSlot Filename))
  (bind _ascharacter_save (Utilities|Casting|CastToCharacterSave _returnvalue)
    (:then
      (bind _outactors (Actor|GetAllActorsOfClass "/Game/ThirdPersonCPP/Blueprints/ThirdPersonCharacter.ThirdPersonCharacter_C"))
      (Variables|Default|SetPlayer (Utilities|Array|Get(acopy) _outactors))
      (Variables|/Game/ThirdPersonCPP/Blueprints/ThirdPersonCharacter.ThirdPersonCharacter_C|SetSkinLoaded (Utilities|Array|Get(acopy) _outactors) true)
      (bind _keys (Utilities|Map|Keys (Variables|/Game/CharacterSave.CharacterSave_C|GetCharacterParts _ascharacter_save)))
      (for _array_element _keys
        (CallFunction|SetSelectedMesh _array_element)
        (CallFunction|SetSkeletalMesh (Variables|Default|GetMesh) (.Mesh (Utilities|Struct|BreakCharacterPartData (.Value (Utilities|Map|Find (Variables|/Game/CharacterSave.CharacterSave_C|GetCharacterParts _ascharacter_save) _array_element)))))
        (CallFunction|SetColor (.Color (Utilities|Struct|BreakCharacterPartData (.Value (Utilities|Map|Find (Variables|/Game/CharacterSave.CharacterSave_C|GetCharacterParts _ascharacter_save) _array_element))))))
      (return true))
    (:CastFailed
      (return false))))

(fn SetSelectedMesh
  (params (NewParam :type CharacterParts%20Enum :default "NewEnumerator0"))
  (bind (_hair _mesh _shirt _shorts _skates _goggles _headphones) (Class|PlayerInterface|GetMeshes(Message) (Game|GetPlayerCharacter 0)))
  (Variables|Default|SetMeshEnum NewParam)
  (Variables|Default|SetMesh (Utilities|Select :Index NewParam :NewEnumerator0 _hair :NewEnumerator1 _mesh :NewEnumerator2 _shirt :NewEnumerator3 _shorts :NewEnumerator4 _skates :NewEnumerator5 _goggles :NewEnumerator6 _headphones :NewEnumerator7 0 :NewEnumerator8 0)))

(fn SetSkeletalMesh
  (params (MeshToChange :type Skeletal%20Mesh%20Component%20Object%20Reference) (NewMesh :type Skeletal%20Mesh%20Object%20Reference))
  (Class|SkinnedMeshComponent|SetSkeletalMesh MeshToChange NewMesh true))

(fn SetColor
  (params (NewParam :type Linear%20Color%20Structure))
  (CallFunction|SetMeshColor NewParam (Variables|Default|GetMesh) (Variables|Default|GetMeshEnum)))

(fn SetMeshColor
  (params (NewParam :type Linear%20Color%20Structure) (MeshToChange :type Skeletal%20Mesh%20Component%20Object%20Reference) (MeshEnum :type CharacterParts%20Enum :default "NewEnumerator0"))
  (Variables|Default|SetMeshEnum MeshEnum)
  (if (Variables|Default|GetIsMale)
    (if (.ReturnValue (Utilities|Map|Find (Variables|Default|GetMaleIndicies) (Variables|Default|GetMeshEnum)))
      (CallFunction|SetGenderedColors MeshToChange NewParam (.Value (Utilities|Map|Find (Variables|Default|GetMaleIndicies) (Variables|Default|GetMeshEnum))))
      (else
        (CallFunction|SetGenderedColors MeshToChange NewParam)))
    (elif (.ReturnValue (Utilities|Map|Find (Variables|Default|GetFemaleIndices) (Variables|Default|GetMeshEnum)))
      (CallFunction|SetGenderedColors MeshToChange NewParam (.Value (Utilities|Map|Find (Variables|Default|GetFemaleIndices) (Variables|Default|GetMeshEnum))))
      (CallFunction|SetGenderedColors MeshToChange NewParam)
      (else
        (CallFunction|SetGenderedColors MeshToChange NewParam)))))

(fn SetGenderedColors
  (params (MeshToChange :type Skeletal%20Mesh%20Component%20Object%20Reference) (NewParam1 :type Linear%20Color%20Structure) (MaterialIndex :type Integer))
  (if (>= MaterialIndex 0)
    (bind _returnvalue (Rendering|Material|CreateDynamicMaterialInstance MeshToChange MaterialIndex (Rendering|Material|GetMaterial MeshToChange MaterialIndex) "None" :!class /Script/Engine.PrimitiveComponent))
    (Rendering|Material|SetVectorParameterValue _returnvalue "Param" NewParam1 :!class /Script/Engine.MaterialInstanceDynamic)
    (else
      (for (_array_element _array_index) (Rendering|Material|GetMaterials MeshToChange)
        (bind _returnvalue_2 (Rendering|Material|CreateDynamicMaterialInstance MeshToChange _array_index _array_element "None" :!class /Script/Engine.PrimitiveComponent))
        (Rendering|Material|SetVectorParameterValue _returnvalue_2 "Param" NewParam1 :!class /Script/Engine.MaterialInstanceDynamic)))))